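; Example pawn for the SKG Attachment system that previews a replicated actor and its attachment customizer UI.
; The server spawns the actor at AttachLocation, and a rep notify rebuilds the W_Customizer widget from its attachment manager for the local player.
; Spawn and destroy requests route through server calls, constructing from deserialized attachment data or clearing the manager.
; Holding right mouse enables movement and look, while the wheel zooms the spring arm within limits.
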(event `InputAxis|MoveUp`
  (params (AxisValue :type "Float (single-precision)"))
  (if (`self.bCanMove`)
    (`self.AddMovementInput` (`self.GetActorUpVector`) (* AxisValue 0.1))))

(event `InputAxis|MoveRight`
  (params (AxisValue :type "Float (single-precision)"))
  (bind _returnvalue (`self.GetActorRightVector`))
  (bind _returnvalue_x (`KismetMathLibrary.BreakVector` (`SceneComponent.GetForwardVector` (`self.Camera`))))
  (if (`self.bCanMove`)
    (if (< _returnvalue_x 0.0)
      (`self.AddMovementInput` _returnvalue (* AxisValue -0.1))
      (else
        (`self.AddMovementInput` _returnvalue (* AxisValue 0.1))))))

(event `self.ReceiveBeginPlay`
  (bind _returnvalue (`GameplayStatics.GetPlayerController` 0))
  (`/Engine/EditorBlueprintResources/ActorMacros.Switch Has Authority`
    (:`Authority`
      (bind _returnvalue_2 (`|SpawnActorFromClass` (`self.ActorClass`) (`SceneComponent.K2_GetComponentToWorld` (`self.AttachLocation`)) "AlwaysSpawn" "OverrideRootScale" self null))
      (set `self.Actor` _returnvalue_2)
      (if (`self.IsLocallyControlled`)
        (set `SpringArmComponent.TargetArmLength` (`self.SpringArmMax`) (`self.SpringArm`))
        (set `PlayerController.bShowMouseCursor` true _returnvalue :!label _label)
        (`WidgetBlueprintLibrary.SetInputMode_GameAndUIEx` _returnvalue null "DoNotLock" false)))
    (:`Remote`
      (goto _label))))

(event `InputAxis|Turn`
  (params (AxisValue :type "Float (single-precision)"))
  (if (`self.bCanMove`)
    (`self.AddControllerYawInput` AxisValue)))

(event `Key|RightMouseButton`
  (params (Key :type "Key Structure"))
  (:`Pressed`
    (bind _output_get (set `self.bCanMove` true)))
  (:`Released`
    (bind _output_get_2 (set `self.bCanMove` false))))

(event `InputAxis|LookUp`
  (params (AxisValue :type "Float (single-precision)"))
  (if (`self.bCanMove`)
    (`self.AddControllerPitchInput` AxisValue)))

(event `Key|MouseScrollUp`
  (params (Key :type "Key Structure"))
  (bind _springarmmin (`self.SpringArmMin`))
  (bind _springarm (`self.SpringArm`))
  (:`Pressed`
    (bind _output_get (set `SpringArmComponent.TargetArmLength` (- (`SpringArmComponent.TargetArmLength` _springarm) (`self.SpringArmAdjustAmount`)) _springarm))
    (if (< _output_get _springarmmin)
      (set `SpringArmComponent.TargetArmLength` _springarmmin (`self.SpringArm`)))))

(event `/Game/SKGAttachment/Blueprints/BP_SpawnActorInterface.SpawnActor`
  (params (DeserializedAttachmentParent :type "SKGAttachmentParent Structure"))
  (`/Engine/EditorBlueprintResources/ActorMacros.Switch Has Authority`
    (:`Authority`
      (`self.SpawnConstructedActor` DeserializedAttachmentParent))
    (:`Remote`
      (`self.Server_SpawnActor` DeserializedAttachmentParent))))

(event `Server_SpawnActor`
  (params (DeserializedAttachmentParent :type "SKGAttachmentParent Structure"))
  (`self.SpawnConstructedActor` DeserializedAttachmentParent))

(event `Key|MouseScrollDown`
  (params (Key :type "Key Structure"))
  (bind _springarmmax (`self.SpringArmMax`))
  (bind _springarm (`self.SpringArm`))
  (:`Pressed`
    (bind _output_get (set `SpringArmComponent.TargetArmLength` (+ (`SpringArmComponent.TargetArmLength` _springarm) (`self.SpringArmAdjustAmount`)) _springarm))
    (if (> _output_get _springarmmax)
      (set `SpringArmComponent.TargetArmLength` _springarmmax (`self.SpringArm`)))))

(event `/Game/SKGAttachment/Blueprints/BP_SpawnActorInterface.DestroyCurrentActor`
  (bind _actor (`self.Actor`))
  (`/Engine/EditorBlueprintResources/StandardMacros.IsValid` _actor
    (:`Is Valid`
      (`/Engine/EditorBlueprintResources/ActorMacros.Switch Has Authority`
        (:`Authority`
          (bind _returnvalue (message `SKGAttachmentInterface.GetAttachmentManager` _actor))
          (`SKGAttachmentManager.DestroyAll` _returnvalue))
        (:`Remote`
          (`self.Server_DestroyCurrentActor`))))))

(event `Server_DestroyCurrentActor`
  (bind _actor (`self.Actor`))
  (`/Engine/EditorBlueprintResources/StandardMacros.IsValid` _actor
    (:`Is Valid`
      (bind _returnvalue (message `SKGAttachmentInterface.GetAttachmentManager` _actor))
      (`SKGAttachmentManager.DestroyAll` _returnvalue))))

(fn `OnRep_Firearm`
  (locals (NewLocalVar_0 :type "/Game/SKGAttachment/Blueprints/UI/Core/W_Customizer Object Reference"))
  (bind _actor (`self.Actor`))
  (bind _w_customizer (`self.W_Customizer`))
  (if (`self.IsLocallyControlled`)
    (`/Engine/EditorBlueprintResources/StandardMacros.IsValid` _w_customizer
      (:`Is Valid`
        (`Widget.RemoveFromParent` _w_customizer))
      (:`Is Not Valid`
        _))
    (`/Engine/EditorBlueprintResources/StandardMacros.IsValid` _actor
      (:`Is Valid`
        (bind _returnvalue (message `SKGAttachmentInterface.GetAttachmentManager` _actor))
        (bind _returnvalue_2 (`|CreateWidget` "/Game/SKGAttachment/Blueprints/UI/Core/W_Customizer.W_Customizer_C" null _returnvalue))
        (bind _output_get (set `self.W_Customizer` _returnvalue_2))
        (`UserWidget.AddToViewport` _output_get 0)))))

(fn `SpawnConstructedActor`
  (params (DeserializedAttachmentParent :type "SKGAttachmentParent Structure"))
  (bind (_error _returnvalue) (`SKGAttachmentFunctionLibrary.ConstructAttachmentParent` self DeserializedAttachmentParent))
  (if (`KismetStringLibrary.IsEmpty` _error)
    (bind _output_get (set `self.Actor` _returnvalue))
    (`self.K2_SetActorTransform` _output_get (`SceneComponent.K2_GetComponentToWorld` (`self.AttachLocation`)) false false)))

(fn `UserConstructionScript`)