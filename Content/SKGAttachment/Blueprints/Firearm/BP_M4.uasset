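; M4 firearm Blueprint that acts as a host for SKG modular attachments.
; Attachment getters expose its SkeletalMesh and SKGAttachmentManager, which supplies the component lists; GetAllAttachmentComponents always passes false, ignoring its ReCache input.
; SetIsLoadedbyPreset stores whether default parts spawn when loading from a preset.
; Offset, overlap, owning-component and typed mesh functions are stubs returning empty, zero or false.
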(event `SKGAttachmentInterface.SetIsLoadedByPreset`
  (set `self.bShouldSpawnDefaultPartsFromPreset` (`self.bSpawnDefaultPartsFromPreset`)))

(fn `AddOffset`
  (params (Offset :type "Float (double-precision)"))
  (returns (ReturnValue :type Boolean))
  (return false))

(fn `GetAllAttachmentComponents`
  (params (bReCache :type Boolean))
  (returns (ReturnValue :type "Array of SKGAttachmentComponent Object Reference"))
  (return (`SKGAttachmentManager.GetAllAttachmentComponents` (`self.SKGAttachmentManager`) false)))

(fn `GetAttachmentAttachOffset`
  (returns (ReturnValue :type "Transform Structure"))
  (return))

(fn `GetAttachmentComponents`
  (returns (ReturnValue :type "Array of SKGAttachmentComponent Object Reference"))
  (return (`SKGAttachmentManager.GetAttachmentComponents` (`self.SKGAttachmentManager`))))

(fn `GetAttachmentManager`
  (returns (ReturnValue :type "SKGAttachmentManager Object Reference"))
  (return (`self.SKGAttachmentManager`)))

(fn `GetAttachmentOffset`
  (returns (ReturnValue :type "Float (double-precision)"))
  (return 0.0))

(fn `GetMesh`
  (returns (ReturnValue :type "MeshComponent Object Reference"))
  (return (`self.SkeletalMesh`)))

(fn `GetMeshSkeletal`
  (returns (ReturnValue :type "SkeletalMeshComponent Object Reference"))
  (return null))

(fn `GetMeshStatic`
  (returns (ReturnValue :type "StaticMeshComponent Object Reference"))
  (return null))

(fn `GetOwningAttachmentComponent`
  (returns (ReturnValue :type "SKGAttachmentComponent Object Reference"))
  (return null))

(fn `GetShouldSpawnDefaultOnPreset`
  (returns (ReturnValue :type Boolean))
  (return (`self.bShouldSpawnDefaultPartsFromPreset`)))

(fn `IsMovementInverted`
  (returns (ReturnValue :type Boolean))
  (return false))

(fn `SetOffset`
  (params (Offset :type "Float (double-precision)"))
  (returns (ReturnValue :type Boolean))
  (return false))

(fn `ShouldBeCheckedForOverlap`
  (returns (ReturnValue :type Boolean))
  (return false))

(fn `UserConstructionScript`)